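; Rain example actor that feeds an orthographic scene capture's view data to a Niagara system.
; Every tick it teleports to its Location variable, then sets the capture's max view distance and switches its render target to nearest filtering.
; It packs the capture's position, axis vectors, ortho width, view distance and near clip plane into one matrix parameter for Niagara.
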(event EventTick
  (params (DeltaSeconds :type Float%20%28single-precision%29))
  ;[0.15 0.15 0.15 0.5] Every Tick
  (Transformation|SetActorLocation (Variables|Default|GetLocation) false true)
  (CallFunction|UpdateNiagara (Variables|Default|GetSceneCapture) (Variables|Default|GetParam) (Variables|Default|GetMaxDistance)))

(fn ConstructionScript)

(fn UpdateNiagara
  (params (Comp :type Scene%20Capture%20Component%202D%20Object%20Reference) (Param :type Name) (MaxDistance :type Float%20%28double-precision%29))
  (bind _returnvalue (Math|Vector|GetForwardVector Comp))
  (bind _returnvalue_2 (Math|Vector|GetUpVector Comp))
  (bind _returnvalue_3 (Math|Vector|GetRightVector Comp))
  (bind _returnvalue_4 (Transformation|GetWorldLocation Comp))
  (bind (_x _y _z) (Math|Vector|BreakVector _returnvalue_4))
  (bind (_x_2 _y_2 _z_2) (Math|Vector|BreakVector _returnvalue))
  (bind (_x_3 _y_3 _z_3) (Math|Vector|BreakVector _returnvalue_3))
  (bind (_x_4 _y_4 _z_4) (Math|Vector|BreakVector _returnvalue_2))
  (bind _output_get (Variables|/Script/Engine.SceneCaptureComponent|SetMaxViewDistanceOverride Comp MaxDistance))
  (Variables|/Script/Engine.Texture|SetFilter (Variables|/Script/Engine.SceneCaptureComponent2D|GetTextureTarget Comp) "TF_Nearest")
  (Class|NiagaraComponent|SetVariableMatrix (Variables|Default|GetNiagara) Param (Utilities|Struct|MakeMatrix (Utilities|Struct|MakePlane (Variables|/Script/Engine.SceneCaptureComponent2D|GetOrthoWidth Comp) _x _y _z) (Utilities|Struct|MakePlane 1.0 _x_3 _y_3 _z_3) (Utilities|Struct|MakePlane _output_get _x_4 _y_4 _z_4) (Utilities|Struct|MakePlane (Variables|/Script/Engine.SceneCaptureComponent2D|GetCustomNearClippingPlane Comp) _x_2 _y_2 _z_2))))